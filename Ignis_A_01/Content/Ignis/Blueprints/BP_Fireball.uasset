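; BP_Fireball is a physics-driven projectile launched along its shooter's FireballDirection by InitShooter, with a cast sound on spawn.
; InnerCollider hits set a Hit flag, ignoring the shooter and actors tagged Fireball.
; Tick counts down its lifetime and destroys it with a positional explosion sound once it hits, nearly stops or times out.
; The file itself applies no damage.
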(event `self.ReceiveBeginPlay`
  (`GameplayStatics.PlaySound2D` "/Game/Ignis/Audio/Fire_Cast.Fire_Cast" 0.5 1.0 0.3 null null))

(event `self.ReceiveTick`
  (params (DeltaSeconds :type "Float (single-precision)"))
  (set `self.TimeAlive` (- (`self.TimeAlive`) DeltaSeconds))
  (bind _returnvalue (`PrimitiveComponent.GetPhysicsLinearVelocity` (`self.Mesh`) "None"))
  (if (or (`self.Hit`) (`KismetMathLibrary.Vector_IsNearlyZero` _returnvalue) (<= (`self.TimeAlive`) 0.0))
    (`GameplayStatics.PlaySoundAtLocation` "/Game/Ignis/Audio/Fire_Explosion.Fire_Explosion" (`SceneComponent.K2_GetComponentLocation` (`self.Mesh`)) (struct) 0.5 1.0 0.0 "/Game/Ignis/Audio/NewSoundAttenuation.NewSoundAttenuation" null null)
    (`self.K2_DestroyActor`)))

(event `self.InnerCollider.OnComponentHit`
  (params (HitComponent :type "PrimitiveComponent Object Reference") (OtherActor :type "Actor Object Reference") (OtherComp :type "PrimitiveComponent Object Reference") (NormalImpulse :type "Vector Structure") (Hit :type "HitResult Structure (by ref)"))
  (bind _shooter (`self.Shooter`))
  (`/Engine/EditorBlueprintResources/StandardMacros.IsValid` _shooter
    (:`Is Valid`
      (if (`KismetMathLibrary.BooleanNOR` (== _shooter OtherActor) (`self.ActorHasTag` OtherActor "Fireball"))
        (set `self.Hit` true)))))

(fn `Init Shooter`
  (params (Shooter :type "/Game/Ignis/Blueprints/ThirdPersonCharacter Object Reference") (Speed :type "Float (double-precision)"))
  (set `self.Shooter` Shooter)
  (`PrimitiveComponent.SetPhysicsLinearVelocity` (`self.Mesh`) (* (`/Game/Ignis/Blueprints/ThirdPersonCharacter.Fireball Direction` Shooter) Speed) false "None"))

(fn `UserConstructionScript`)