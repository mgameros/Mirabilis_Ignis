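; BP_Ice is an ice block that vanishes when hit by a Fireball-tagged actor or component, switching its mesh to hidden and overlap-only.
; A Tick countdown from RespawnTime reforms it, waiting until the player stops overlapping; a zero time disables automatic reforming.
; An external RespawnIce event can also restore it immediately.
; It registers with linked MovingPlatforms on BeginPlay and notifies them when destroyed.
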(event `self.ReceiveActorBeginOverlap`
  (params (OtherActor :type "Actor Object Reference"))
  ;[1 1 1] Actor touching
  (if (`self.ActorHasTag` OtherActor "Player")
    (set `self.touching` true)))

(event `self.ReceiveBeginPlay`
  (for _array_element (`self.platform`)
    (bind _asmoving_platform (cast `/Game/Ignis/Blueprints/MovingPlatform` _array_element))
    (`/Game/Ignis/Blueprints/MovingPlatform.AddIceBlock` _asmoving_platform self)))

(event `self.ReceiveActorEndOverlap`
  (params (OtherActor :type "Actor Object Reference"))
  (bind _mesh (`self.Mesh`))
  ;[1 1 1] Actor no longer touching
  (if (`self.ActorHasTag` OtherActor "Player")
    (set `self.touching` false)
    (if (== (`self.respawnTime`) 0.0)
      _
      (elif (<= (`self.respawnLeft`) 0.0)
        ;[1 1 1] Make Solid
        (`PrimitiveComponent.SetCollisionResponseToAllChannels` _mesh "ECR_Block" :!label _label)
        (`SceneComponent.SetVisibility` _mesh true true)))))

(event `RespawnIce`
  (goto _label))

(event `self.ReceiveTick`
  (params (DeltaSeconds :type "Float (single-precision)"))
  (bind _respawnleft (`self.respawnLeft`))
  ;[1 1 1] Reform
  (if (> _respawnleft 0.0)
    (bind _output_get (set `self.respawnLeft` (- _respawnleft DeltaSeconds)))
    (if (<= _output_get 0.0)
      ;[1 1 1] Make Solid
      (if (not (`self.touching`))
        (goto _label)))))

(event `self.ReceiveHit`
  (params (MyComp :type "PrimitiveComponent Object Reference") (Other :type "Actor Object Reference") (OtherComp :type "PrimitiveComponent Object Reference") (bSelfMoved :type Boolean) (HitLocation :type "Vector Structure") (HitNormal :type "Vector Structure") (NormalImpulse :type "Vector Structure") (Hit :type "HitResult Structure (by ref)"))
  (bind _mesh (`self.Mesh`))
  ;[1 1 1] Despawn on Fireball Hit
  (if (or (`self.ActorHasTag` Other "Fireball") (`ActorComponent.ComponentHasTag` OtherComp "Fireball"))
    (set `self.respawnLeft` (`self.respawnTime`))
    (`PrimitiveComponent.SetCollisionResponseToAllChannels` _mesh "ECR_Overlap")
    (`SceneComponent.SetVisibility` _mesh false true)
    (for _array_element (`self.platform`)
      (bind _asmoving_platform (cast `/Game/Ignis/Blueprints/MovingPlatform` _array_element))
      (`/Game/Ignis/Blueprints/MovingPlatform.IceDestroyed` _asmoving_platform))))

(fn `UserConstructionScript`)