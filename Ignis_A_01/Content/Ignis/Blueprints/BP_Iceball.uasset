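; BP_Iceball is a physics-driven projectile that kills the ThirdPersonCharacter when its mesh overlaps the character's capsule.
; InitShooter stores the shooter and launches the mesh in a straight aim at a raised point above that shooter's target character.
; InnerCollider hits flag impact, ignoring the shooter and other iceballs.
; Tick destroys it on impact, near-zero velocity or lifetime expiry.
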(event `self.ReceiveBeginPlay`)

(event `self.ReceiveTick`
  (params (DeltaSeconds :type "Float (single-precision)"))
  (set `self.TimeAlive` (- (`self.TimeAlive`) DeltaSeconds))
  (bind _returnvalue (`PrimitiveComponent.GetPhysicsLinearVelocity` (`self.Mesh`) "None"))
  (if (or (`self.Hit`) (`KismetMathLibrary.Vector_IsNearlyZero` _returnvalue) (<= (`self.TimeAlive`) 0.0))
    (`self.K2_DestroyActor`)))

(event `self.InnerCollider.OnComponentHit`
  (params (HitComponent :type "PrimitiveComponent Object Reference") (OtherActor :type "Actor Object Reference") (OtherComp :type "PrimitiveComponent Object Reference") (NormalImpulse :type "Vector Structure") (Hit :type "HitResult Structure (by ref)"))
  (bind _shooter (`self.Shooter`))
  (`/Engine/EditorBlueprintResources/StandardMacros.IsValid` _shooter
    (:`Is Valid`
      (if (`KismetMathLibrary.BooleanNOR` (== _shooter OtherActor) (`self.ActorHasTag` OtherActor "Iceball"))
        (set `self.Hit` true)))))

(event `self.Mesh.OnComponentBeginOverlap`
  (params (OverlappedComponent :type "PrimitiveComponent Object Reference") (OtherActor :type "Actor Object Reference") (OtherComp :type "PrimitiveComponent Object Reference") (OtherBodyIndex :type Integer) (bFromSweep :type Boolean) (SweepResult :type "HitResult Structure (by ref)"))
  (bind _asthird_person_character (cast `/Game/Ignis/Blueprints/ThirdPersonCharacter` OtherActor))
  (if (== (`Character.CapsuleComponent` _asthird_person_character) OtherComp)
    (`/Game/Ignis/Blueprints/ThirdPersonCharacter.KillPlayer` _asthird_person_character)
    (set `self.Hit` true)))

(fn `Init Shooter`
  (params (Shooter :type "/Game/Ignis/Blueprints/IceMage Object Reference") (Speed :type "Float (double-precision)"))
  (bind _capsulecomponent (`Character.CapsuleComponent` (`/Game/Ignis/Blueprints/IceMage.ThirdPersonCharacter` Shooter)))
  (set `self.Shooter` Shooter)
  (`PrimitiveComponent.SetPhysicsLinearVelocity` (`self.Mesh`) (* (`KismetMathLibrary.Normal` (- (+ (`SceneComponent.K2_GetComponentLocation` _capsulecomponent) (`KismetMathLibrary.MakeVector` 0.0 0.0 (* (`CapsuleComponent.CapsuleHalfHeight` _capsulecomponent) 1.25))) (`SceneComponent.K2_GetComponentLocation` (`self.Mesh`)))) Speed) false "None"))

(fn `UserConstructionScript`)