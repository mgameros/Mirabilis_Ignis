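; IceMage is an enemy that travels a list of waypoints and kills the player on contact with its box trigger.
; Init stores the start point, waypoints and player reference, then calls Respawn to move the cube to the start and reset progress.
; Tick counts down distance by speed, setting physics velocity and yaw toward each next waypoint until the list ends.
; Respawn skips one tick through a flag marked for deletion.
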(event `self.ReceiveTick`
  (params (DeltaSeconds :type "Float (single-precision)"))
  (bind _cube (`self.Cube`))
  (bind _returnvalue (- (`|GetArrayItem` (`self.Locations`) (`self.LocationIndex`)) (`SceneComponent.K2_GetComponentLocation` (`self.Cube`))))
  (bind _returnvalue_2 (`KismetMathLibrary.Normal` _returnvalue))
  (if (`self.Respawned`)
    (set `self.Respawned` false) ; TODO: Delete
    (elif (`self.Done`)
      _
      (elif (> (`self.LocationDistance`) 0.0)
        (set `self.LocationDistance` (- (`self.LocationDistance`) (* (`self.Speed`) DeltaSeconds)))
        (else
          (bind _output_get (set `self.LocationIndex` (+ (`self.LocationIndex`) 1)))
          (if (>= _output_get (`KismetArrayLibrary.Array_Length` (`self.Locations`)))
            (set `self.Done` true)
            (else
              (set `self.LocationDistance` (`KismetMathLibrary.VSize` _returnvalue))
              (`PrimitiveComponent.SetPhysicsLinearVelocity` _cube (* _returnvalue_2 (`self.Speed`)) false "None")
              (`SceneComponent.K2_SetWorldRotation` _cube (`KismetMathLibrary.MakeRotator` 0.0 0.0 (.yaw (`KismetMathLibrary.Conv_VectorToRotator` _returnvalue_2))) false false))))))))

(event `self.Box.OnComponentBeginOverlap`
  (params (OverlappedComponent :type "PrimitiveComponent Object Reference") (OtherActor :type "Actor Object Reference") (OtherComp :type "PrimitiveComponent Object Reference") (OtherBodyIndex :type Integer) (bFromSweep :type Boolean) (SweepResult :type "HitResult Structure (by ref)"))
  (bind _asthird_person_character (cast `/Game/Ignis/Blueprints/ThirdPersonCharacter` OtherActor))
  (`/Game/Ignis/Blueprints/ThirdPersonCharacter.KillPlayer` _asthird_person_character))

(fn `Init`
  (params (StartLocation :type "Vector Structure") (Locations :type "Array of Vector Structure") (ThirdPersonCharacter :type "/Game/Ignis/Blueprints/ThirdPersonCharacter Object Reference"))
  (set `self.StartLocation` StartLocation)
  (set `self.Locations` Locations)
  (set `self.ThirdPersonCharacter` ThirdPersonCharacter)
  (`self.Respawn`))

(fn `Respawn`
  (`SceneComponent.K2_SetWorldLocation` (`self.Cube`) (`self.StartLocation`) false false)
  (set `self.Respawned` true)
  (set `self.LocationIndex` -1)
  (set `self.LocationDistance` -1.0))

(fn `UserConstructionScript`)