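; IceMageDialogue is the Ice Mage actor that starts a dialogue when the third-person character walks into its collision.
; An overlap on DialogueCollision passes the character to the DialogueComponentIceMage component's OnInteraction.
; Helper functions switch the skeletal mesh between looping idle and emote animations.
; DeleteDialogue destroys both the dialogue component and its collision, removing the interaction.
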(event `self.DialogueCollision.OnComponentBeginOverlap`
  (params (OverlappedComponent :type "PrimitiveComponent Object Reference") (OtherActor :type "Actor Object Reference") (OtherComp :type "PrimitiveComponent Object Reference") (OtherBodyIndex :type Integer) (bFromSweep :type Boolean) (SweepResult :type "HitResult Structure (by ref)"))
  (bind _asthird_person_character (cast `/Game/Ignis/Blueprints/ThirdPersonCharacter` OtherActor))
  (`/Game/Ignis/Dialogue/DialogueComponent_IceMage.OnInteraction` (`self.DialogueComponent_IceMage`) _asthird_person_character))

(fn `DeleteDialogue`
  (`ActorComponent.K2_DestroyComponent` (`self.DialogueComponent_IceMage`))
  (`ActorComponent.K2_DestroyComponent` (`self.DialogueCollision`)))

(fn `IceMageEmote`
  (`SkeletalMeshComponent.PlayAnimation` (`self.SkeletalMesh`) "/Game/Ignis/Art+Anims/IceMage/IceMage_Anim_Emote.IceMage_Anim_Emote" true))

(fn `IceMageIdle`
  (`SkeletalMeshComponent.PlayAnimation` (`self.SkeletalMesh`) "/Game/Ignis/Art+Anims/IceMage/IceMage_Anim_Idle.IceMage_Anim_Idle" true))

(fn `UserConstructionScript`)