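; Spawner that creates an Ice Mage for a given player, only when that player has no valid one.
; SpawnIceMage records the player, spawns the mage at the StartLocation actor and stores it on the player's IceMage reference.
; It appends the Locations actors' positions to VectorLocations without clearing it, then passes them, the start position and the player to the mage's Init.
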(fn `SpawnIceMage`
  (params (Player :type "/Game/Ignis/Blueprints/ThirdPersonCharacter Object Reference"))
  (bind _lastplayer (`self.LastPlayer`))
  (bind _returnvalue (`self.K2_GetActorLocation` (`self.Start Location`)))
  (bind _output_get (set `self.LastPlayer` Player))
  (`/Engine/EditorBlueprintResources/StandardMacros.IsValid` (`/Game/Ignis/Blueprints/ThirdPersonCharacter.IceMage` _output_get)
    (:`Is Not Valid`
      (bind _returnvalue_2 (`|SpawnActorFromClass` "/Game/Ignis/Blueprints/IceMage.IceMage_C" (`KismetMathLibrary.MakeTransform` _returnvalue) "Undefined" "OverrideRootScale" null null))
      (bind _output_get_2 (set `/Game/Ignis/Blueprints/ThirdPersonCharacter.IceMage` _returnvalue_2 _lastplayer))
      (for _array_element (`self.Locations`)
        (`KismetArrayLibrary.Array_Add` (`self.VectorLocations`) (`self.K2_GetActorLocation` _array_element)))
      (`/Game/Ignis/Blueprints/IceMage.Init` _output_get_2 _returnvalue (`self.VectorLocations`) _lastplayer))))

(fn `UserConstructionScript`)