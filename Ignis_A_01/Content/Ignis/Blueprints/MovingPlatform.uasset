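; Moving platform Blueprint that shuttles its Cube back and forth between its starting position and an EndPoint component.
; On BeginPlay it caches both world locations and sets the timeline play rate to the inverse of Duration, so Duration controls travel time.
; The timeline lerps the Cube's location without sweep, and each finish flips MoveDirection to alternate between Reverse and Play, looping indefinitely.
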(event `self.ReceiveBeginPlay`
  (bind _movedirection (`self.MoveDirection`))
  (`TimelineComponent.SetPlayRate` (`self.Timeline_0`) (/ 1.0 (`self.Duration`)))
  (bind _output_get (set `self.StartLocation` (`SceneComponent.K2_GetComponentLocation` (`self.Cube`))))
  (bind _output_get_2 (set `self.EndLocation` (`SceneComponent.K2_GetComponentLocation` (`self.EndPoint`))))
  (bind (_direction _newtrack_0) (`Timeline|Timeline_0` :!label _label)
    (:`Update`
      (`SceneComponent.K2_SetWorldLocation` (`self.Cube`) (`KismetMathLibrary.VLerp` _output_get _output_get_2 _newtrack_0) false false))
    (:`Finished`
      (set `self.MoveDirection` (not _movedirection))
      (if _movedirection
        (goto _label :!via `Reverse`)
        (else
          (goto _label))))))

(fn `UserConstructionScript`)