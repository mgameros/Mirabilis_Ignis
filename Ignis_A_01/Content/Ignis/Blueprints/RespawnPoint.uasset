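; Checkpoint actor that updates the player's respawn location and activates a linked mana crystal.
; When a ThirdPersonCharacter overlaps the actor, it passes the collision box's world location to that character's SetRespawnPoint.
; It then calls Activate on the stored ManaCrystal, which is assigned through the AddCrystal event.
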(event `Add Crystal`
  (params (Crystal :type "Actor Object Reference"))
  (set `self.Crystal` Crystal))

(event `self.ReceiveActorBeginOverlap`
  (params (OtherActor :type "Actor Object Reference"))
  (set `self.OtherObject` OtherActor)
  (bind _asthird_person_character (cast `/Game/Ignis/Blueprints/ThirdPersonCharacter` (`self.OtherObject`)))
  (`/Game/Ignis/Blueprints/ThirdPersonCharacter.Set Respawn Point` _asthird_person_character (`SceneComponent.K2_GetComponentLocation` (`self.CollisionBox`)))
  (bind _asmana_crystal (cast `/Game/Ignis/Blueprints/ManaCrystal` (`self.Crystal`)))
  (`/Game/Ignis/Blueprints/ManaCrystal.Activate` _asmana_crystal))

(fn `UserConstructionScript`)