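; BP_TrappedNPC2 is a dialogue NPC, a pyro mage trapped in a crystal cage that can open.
; Separate functions loop the mage's idle or emote animation and play one-shot opening animations on the cage and two crystal meshes.
; Another function destroys the DialogueComponent to remove the dialogue.
; The Blueprint has an empty construction script and never calls these functions itself.
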(fn `CageOpen`
  (`SkeletalMeshComponent.PlayAnimation` (`self.Cage`) "/Game/Ignis/Art+Anims/Cage/Cage_Cage_Topper_Anim_Open.Cage_Cage_Topper_Anim_Open" false)
  (`SkeletalMeshComponent.PlayAnimation` (`self.Crystals`) "/Game/Ignis/Art+Anims/Cage/Cage_Large_Crystal_Anim_Open.Cage_Large_Crystal_Anim_Open" false)
  (`SkeletalMeshComponent.PlayAnimation` (`self.Crystals2`) "/Game/Ignis/Art+Anims/Cage/Cage_Large_Crystal5_Anim_Open.Cage_Large_Crystal5_Anim_Open" false))

(fn `DeleteDialogue`
  (`ActorComponent.K2_DestroyComponent` (`self.DialogueComponent`)))

(fn `PyroEmote`
  (`SkeletalMeshComponent.PlayAnimation` (`self.Mesh`) "/Game/Ignis/Art+Anims/PyroMage/PyroMage_Anim_Emote.PyroMage_Anim_Emote" true))

(fn `PyroIdle`
  (`SkeletalMeshComponent.PlayAnimation` (`self.Mesh`) "/Game/Ignis/Art+Anims/PyroMage/PyroMage_Anim_Idle.PyroMage_Anim_Idle" true))

(fn `UserConstructionScript`)